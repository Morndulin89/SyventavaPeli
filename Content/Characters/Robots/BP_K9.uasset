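; K9 robot character that follows the player via AI MoveTo and holds branching conversations on sphere overlap when in its Dialogue action.
; ACDialogtree runs the text-file dialogue; response tags record the player's name, goal, nickname and attitude.
; A fixed-length circular memory of friendly/hostile responses sets the attitude score, which selects the next dialogue file.
; Steering-behavior switch and facing/range check are present but disconnected.
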(event `self.ReceiveBeginPlay`
  (bind _asw_robot_hud (cast `/Game/Characters/Robots/W_RobotHud` (`WidgetComponent.GetUserWidgetObject` (`self.Widget`))))
  (set `/Game/Characters/Robots/W_RobotHud.Owner` self _asw_robot_hud))

(event `self.ReceiveTick`
  (params (DeltaSeconds :type "Float (single-precision)"))
  (bind _returnvalue (`GameplayStatics.GetPlayerCharacter` 0))
  (`/Engine/EditorBlueprintResources/StandardMacros.DoOnce` false :!label _label
    (:`Completed`
      (if (`KismetSystemLibrary.IsValid` _returnvalue)
        (`|AIMoveTo` self (0.0 0.0 0.0) _returnvalue
          (:`OnSuccess`
            (goto _label :!via `Reset`)))))))

(event `self.Sphere.OnComponentBeginOverlap`
  (params (OverlappedComponent :type "PrimitiveComponent Object Reference") (OtherActor :type "Actor Object Reference") (OtherComp :type "PrimitiveComponent Object Reference") (OtherBodyIndex :type Integer) (bFromSweep :type Boolean) (SweepResult :type "HitResult Structure (by ref)"))
  (bind _ac_dialogtree (`self.AC_Dialogtree`))
  ;[1 1 1] Discussion
  (if (`self.ActorHasTag` OtherActor "Player")
    (if (`|EnumEquality` (`self.CurrentAction`) "NewEnumerator8")
      ;;[1 1 1] If conversation has started already
      (if (== (`self.CurrentAIPhrase`) 0)
        ;;[1 1 1] Set up the dialogue tree and update the current AI phrase
        (`/Game/Characters/Robots/AI_Components/dialogueTree/AC_Dialogtree.SetUpDialogTree` _ac_dialogtree (`self.ActiveDiscussionFileName`))
        (set `self.CurrentAIPhrase` (`/Game/Characters/Robots/AI_Components/dialogueTree/AC_Dialogtree.CurrentAIPhraseID` _ac_dialogtree))
        (if (`KismetSystemLibrary.IsValid` (`/Game/Characters/Robots/AI_Components/dialogueTree/AC_Dialogtree.DialogHud` _ac_dialogtree))
          ;;[1 1 1] Bind event to handle AI's responses based on the event dispatched by GUI when player speaks
          (add `/Game/Characters/Robots/AI_Components/dialogueTree/W_DialogueHUD.ED_PlayerSpoke` (`/Game/Characters/Robots/AI_Components/dialogueTree/AC_Dialogtree.DialogHud` (`self.AC_Dialogtree`)) (delegate `PlayerSpoke`)))))))

(event `PlayerSpoke`
  (params (NewParam :type Integer))
  (bind _ac_dialogtree (`self.AC_Dialogtree`))
  (bind (_name _attitude) (break `/Game/Characters/Robots/AI_Components/dialogueTree/S_PlayerInfo` (`self.PlayerInfo`)))
  ;[1 1 1] Discussion
  ;;[1 1 1] After every response of the player update the tree...
  (bind (_responsetag _responseinfo _nextnode) (`/Game/Characters/Robots/AI_Components/dialogueTree/AC_Dialogtree.UpdateTree` (`self.AC_Dialogtree`) NewParam))
  ;;[1 1 1] Check the info from the discussion
  (`self.ProcessDiscussionInfo` _responsetag _responseinfo)
  ;;[1 1 1] ... check if conversation continues and update the current phrase...
  (if (> _nextnode 0)
    (set `self.CurrentAIPhrase` (`/Game/Characters/Robots/AI_Components/dialogueTree/AC_Dialogtree.CurrentAIPhraseID` _ac_dialogtree))
    (else
      ;;[1 1 1] or disable the dialogue tree and update attitude towards player
      (`/Game/Characters/Robots/AI_Components/dialogueTree/AC_Dialogtree.DisableDialogTree` _ac_dialogtree)
      (`self.UpdateAttitudeTowardsPlayer`)
      ;;[1 1 1] Update text file based on the attitude towards player
      (if true
        (if (>= _attitude 0.1)
          (set `self.ActiveDiscussionFileName` "Dialog3.txt")
          (elif (> _attitude -0.1)
            (set `self.ActiveDiscussionFileName` "Dialog2.txt")))))))

(event `self.Sphere.OnComponentEndOverlap`
  (params (OverlappedComponent :type "PrimitiveComponent Object Reference") (OtherActor :type "Actor Object Reference") (OtherComp :type "PrimitiveComponent Object Reference") (OtherBodyIndex :type Integer))
  ;[1 1 1] Discussion
  ;;[1 1 1] When player goes away....
  (if (`self.ActorHasTag` OtherActor "Player")
    ;;;[1 1 1] ...disable dialogHUD and reset AIPhrase
    (`/Game/Characters/Robots/AI_Components/dialogueTree/AC_Dialogtree.DisableDialogTree` (`self.AC_Dialogtree`))
    (set `self.CurrentAIPhrase` 0)))

(fn `IsWithinDiscussionRange`
  (returns (Result :type Boolean))
  (locals (MinDiscussionRange :type "Float (double-precision)" :default -0.5) (MaxDiscussionRange :type "Float (double-precision)" :default -0.25) (MaxDiscussionAngle :type "Float (double-precision)" :default 90.0))
  (bind _returnvalue (`KismetMathLibrary.Conv_RotatorToVector` (`self.K2_GetActorRotation`)))
  (bind _returnvalue_2 (`KismetMathLibrary.Conv_RotatorToVector` (`self.K2_GetActorRotation` (`GameplayStatics.GetPlayerCharacter` 0))))
  (return (and (< (`KismetMathLibrary.Dot_VectorVector` (`self.GetActorForwardVector`) (`KismetMathLibrary.Normal` (- (`self.K2_GetActorLocation`) (`self.K2_GetActorLocation` (`GameplayStatics.GetPlayerCharacter` 0))))) (`KismetMathLibrary.DegCos` (`local.MaxDiscussionAngle`))) (`KismetMathLibrary.InRange_FloatFloat` (/ (`KismetMathLibrary.Dot_VectorVector` _returnvalue _returnvalue_2) (+ (`KismetMathLibrary.VSize` _returnvalue) (`KismetMathLibrary.VSize` _returnvalue_2))) (`local.MinDiscussionRange`) (`local.MaxDiscussionRange`)) (< (`KismetMathLibrary.Vector_Distance` (`self.K2_GetActorLocation`) (`self.K2_GetActorLocation` (`GameplayStatics.GetPlayerCharacter` 0))) (`self.DiscussionRange`)))))

(fn `ProcessDiscussionInfo`
  (params (Tag :type String) (Info :type String))
  (bind _playerinfo (`self.PlayerInfo`))
  (bind _information (`self.Information`))
  (bind _shorttermplayerattitude (`self.ShortTermPlayerAttitude`))
  (bind _shorttermplayerattitude_2 (`self.ShortTermPlayerAttitude`))
  (bind _information_2 (`self.Information`))
  (bind _returnvalue (`KismetStringLibrary.ParseIntoArray` (`self.Information`) ":"))
  (bind _output (`|GetArrayItem` _returnvalue))
  (set `self.Information` Info)
  (switch `string` Tag
    (:`PC_NAME`
      ;[1 1 1] Update info based on discussion
      (setmembers `/Game/Characters/Robots/AI_Components/dialogueTree/S_PlayerInfo` :`StructRef` _playerinfo :`Name` _information))
    (:`PC_GOAL`
      (setmembers `/Game/Characters/Robots/AI_Components/dialogueTree/S_PlayerInfo` :`StructRef` _playerinfo :`Goal` _information))
    (:`PC_ATTITUDE`
      ;[1 1 1] Insert new evidence of player attitude into fixed short-term memory
      (if (< (`KismetArrayLibrary.Array_Length` (`self.ShortTermPlayerAttitude`)) (`self.ShortTermMemoryLength`))
        (bind _returnvalue_2 (`KismetArrayLibrary.Array_Add` (`self.ShortTermPlayerAttitude`) _information_2))
        (set `self.IndexToAddToMemory` (+ _returnvalue_2 1))
        (else
          (if (< (`self.IndexToAddToMemory`) (`self.ShortTermMemoryLength`))
            (`KismetArrayLibrary.Array_Set` _shorttermplayerattitude (`self.IndexToAddToMemory`) _information_2)
            (else
              (bind _output_get (set `self.IndexToAddToMemory` 0))
              (`KismetArrayLibrary.Array_Set` _shorttermplayerattitude _output_get _information_2)))
          (`/Engine/EditorBlueprintResources/StandardMacros.IncrementInt` (`self.IndexToAddToMemory`)))))
    (:`PC_ATTITUDE_AND_NICKNAME`
      ;[1 1 1] Insert new evidence of player attitude into the short-term memory
      (setmembers `/Game/Characters/Robots/AI_Components/dialogueTree/S_PlayerInfo` :`StructRef` (`self.PlayerInfo`) :`Nickname` (`|GetArrayItem` _returnvalue 1))
      (if (< (`KismetArrayLibrary.Array_Length` (`self.ShortTermPlayerAttitude`)) (`self.ShortTermMemoryLength`))
        (bind _returnvalue_3 (`KismetArrayLibrary.Array_Add` (`self.ShortTermPlayerAttitude`) _output))
        (set `self.IndexToAddToMemory` (+ _returnvalue_3 1))
        (else
          (if (< (`self.IndexToAddToMemory`) (`self.ShortTermMemoryLength`))
            (`KismetArrayLibrary.Array_Set` _shorttermplayerattitude_2 (`self.IndexToAddToMemory`) _output)
            (else
              (bind _output_get_2 (set `self.IndexToAddToMemory` 0))
              (`KismetArrayLibrary.Array_Set` _shorttermplayerattitude_2 _output_get_2 _output)))
          (`/Engine/EditorBlueprintResources/StandardMacros.IncrementInt` (`self.IndexToAddToMemory`)))))))

(fn `UpdateAttitudeTowardsPlayer`
  (locals (PositiveMemories :type Integer) (NegativeMemories :type Integer))
  (bind _returnvalue (`KismetMathLibrary.Conv_IntToDouble` (/ (`local.PositiveMemories`) (+ (`local.PositiveMemories`) (`local.NegativeMemories`)))))
  ;[1 1 1] Calculate number of positive and negative short-term memories
  (for _array_element (`self.ShortTermPlayerAttitude`)
    (if (== _array_element "FRIENDLY")
      (`/Engine/EditorBlueprintResources/StandardMacros.IncrementInt` (`local.PositiveMemories`))
      (elif (== _array_element "HOSTILE")
        (`/Engine/EditorBlueprintResources/StandardMacros.IncrementInt` (`local.NegativeMemories`)))))
  ;[1 1 1] If there are any positive or negative memories...
  (if (or (> (`local.PositiveMemories`) 0) (> (`local.NegativeMemories`) 0))
    ;[1 1 1] Calculate ratio between positive and negative short-term memories and save it as a percentage towards the player
    (setmembers `/Game/Characters/Robots/AI_Components/dialogueTree/S_PlayerInfo` :`StructRef` (`self.PlayerInfo`) :`Attitude` _returnvalue)
    ;[1 1 1] apuprintstringit
    (`KismetSystemLibrary.PrintString` (`KismetStringLibrary.Concat_StrStr` "Positive: " (`KismetStringLibrary.Conv_IntToString` (`local.PositiveMemories`))))
    (`KismetSystemLibrary.PrintString` (`KismetStringLibrary.Concat_StrStr` "Negative: " (`KismetStringLibrary.Conv_IntToString` (`local.NegativeMemories`))))
    (`KismetSystemLibrary.PrintString` (`KismetStringLibrary.Concat_StrStr` "Percentage: " (`KismetStringLibrary.Conv_DoubleToString` _returnvalue)))
    (for _array_element_2 (`self.ShortTermPlayerAttitude`)
      (`KismetSystemLibrary.PrintString` _array_element_2))))

(fn `UserConstructionScript`)