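; BP_DalekFlocking is a Dalek robot character whose movement each tick is driven by its current behaviour state.
; A switch on CurrentAction hands the CharacterMovement component to a matching steering component: idle, seek, face, path following, flee or path with stop.
; Behaviours that react to the player also receive the player's movement component.
; In Flocking, it rotates toward the player before the flock component computes its new position, and prints that direction.
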(event `self.ReceiveTick`
  (params (DeltaSeconds :type "Float (single-precision)"))
  (bind _returnvalue (- (`CharacterMovementComponent.GetLastUpdateLocation` (`Character.CharacterMovement` (`GameplayStatics.GetPlayerCharacter` 0))) (`CharacterMovementComponent.GetLastUpdateLocation` (`self.CharacterMovement`))))
  (if (`|EnumEquality` (`self.CurrentAction`) "NewEnumerator6")
    (`KismetSystemLibrary.PrintString` (`KismetStringLibrary.Conv_VectorToString` _returnvalue))
    ;[1 1 1] if current behaviour is set to flocking, calculate the flocking velocity and set position seeking to flocking
    (bind _output_get (set `self.velocityForFlocking` _returnvalue))
    (`self.K2_SetActorRotation` (`KismetMathLibrary.Conv_VectorToRotator` _output_get))
    (`/Game/Characters/Robots/AI_Components/SteeringBehaviour/AC_Flock.calculateNewPosition` (`self.AC_Flock`) (`self.CharacterMovement`))
    (else
      (switch `/Game/Characters/Robots/AI_Components/SteeringBehaviour/E_Behaviours` (`self.CurrentAction`)
        (:`NewEnumerator0`
          ;[1 1 1] Idle
          (`/Game/Characters/Robots/AI_Components/SteeringBehaviour/AC_Idle.calculateNewPosition` (`self.AC_Idle`) (`self.CharacterMovement`)))
        (:`NewEnumerator1`
          ;[1 1 1] Seek the player
          (`/Game/Characters/Robots/AI_Components/SteeringBehaviour/AC_Seek.calculateNewPosition` (`self.AC_Seek`) (`self.CharacterMovement`) (`Character.CharacterMovement` (`GameplayStatics.GetPlayerCharacter` 0))))
        (:`NewEnumerator2`
          ;[1 1 1] Face the character
          (`/Game/Characters/Robots/AI_Components/SteeringBehaviour/AC_Face.calculateNewPosition` (`self.AC_Face`) (`self.CharacterMovement`) (`Character.CharacterMovement` (`GameplayStatics.GetPlayerCharacter` 0))))
        (:`NewEnumerator3`
          ;[1 1 1] Follow along specified path
          (`/Game/Characters/Robots/AI_Components/SteeringBehaviour/AC_FollowPath.calculateNewPosition` (`self.AC_FollowPath`) (`self.CharacterMovement`)))
        (:`NewEnumerator4`
          ;[1 1 1] Flee player
          (`/Game/Characters/Robots/AI_Components/SteeringBehaviour/AC_Flee.calculateNewPosition` (`self.AC_Flee`) (`self.CharacterMovement`) (`Character.CharacterMovement` (`GameplayStatics.GetPlayerCharacter` 0)))
          (set `self.isFleeing` true))
        (:`NewEnumerator5`
          ;[1 1 1] Path with stop
          (`/Game/Characters/Robots/AI_Components/SteeringBehaviour/AC_FollowPathWithStop.calculateNewPosition` (`self.AC_FollowPathWithStop`) (`self.CharacterMovement`) (`Character.CharacterMovement` (`GameplayStatics.GetPlayerCharacter` 0))))))))

(fn `UserConstructionScript`)