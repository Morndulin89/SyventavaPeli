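; Dialogue tree component that runs branching conversations between an AI and the player, with up to three responses.
; Setup creates the HUD, enables mouse input and parses a semicolon-delimited file into a flat array.
; UpdateTree follows next-phrase IDs using five-field index math, hides "-" choices and returns the response's tag, info and next node, zero meaning end.
; DisableDialogTree removes the HUD and restores game-only input.
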(fn `DisableDialogTree`
  (bind _returnvalue (`GameplayStatics.GetPlayerController` 0))
  (bind _dialoghud (`self.DialogHud`))
  (if (`KismetSystemLibrary.IsValid` _dialoghud)
    (`Widget.RemoveFromParent` _dialoghud)
    (`WidgetBlueprintLibrary.SetInputMode_GameOnly` _returnvalue)
    (set `PlayerController.bShowMouseCursor` false _returnvalue)
    (set `self.CurrentAIPhraseID` 0)))

(fn `GetGUIVariables`
  (bind _dialoghud (`self.DialogHud`))
  (set `self.TXT AIText` (`/Game/Characters/Robots/AI_Components/dialogueTree/W_DialogueHUD.TXT_AIText` _dialoghud))
  (set `self.TXT Char Choice 1` (`/Game/Characters/Robots/AI_Components/dialogueTree/W_DialogueHUD.TXT_CharChoice1` _dialoghud))
  (set `self.TXT Char Choice 2` (`/Game/Characters/Robots/AI_Components/dialogueTree/W_DialogueHUD.TXT_CharChoice2` _dialoghud))
  (set `self.TXT Char Choice 3` (`/Game/Characters/Robots/AI_Components/dialogueTree/W_DialogueHUD.TXT_CharChoice3` _dialoghud)))

(fn `SetUpDialogTree`
  (params (DialogFile :type String))
  (bind _returnvalue (`GameplayStatics.GetPlayerController` 0))
  (bind _output (`|GetArrayItem` (`self.DialogArray`) 16))
  (bind _output_2 (`|GetArrayItem` (`self.DialogArray`) 6))
  (bind _output_3 (`|GetArrayItem` (`self.DialogArray`) 11))
  ;[1 1 1] Check the tree for the dialog is valid and set it up
  (set `self.Dialog File` DialogFile)
  (if (`KismetStringLibrary.Contains` DialogFile "Dialog")
    ;[1 1 1] Create dialog tree HUD and add it to viewport
    (bind _returnvalue_2 (`|CreateWidget` "/Game/Characters/Robots/AI_Components/dialogueTree/W_DialogueHUD.W_DialogueHUD_C"))
    (bind _output_get (set `self.DialogHud` _returnvalue_2))
    (`UserWidget.AddToViewport` _output_get 0)
    ;[1 1 1] Show the widget
    (`self.ShowAnswerGUIWidgets`)
    ;[1 1 1] Get variables from GUI
    (`self.GetGUIVariables`)
    ;[1 1 1] Set inputmode and show mouse cursor
    (`WidgetBlueprintLibrary.SetInputMode_GameAndUIEx` _returnvalue null)
    (set `PlayerController.bShowMouseCursor` true _returnvalue)
    ;[1 1 1] Get the dialog from the file and parse it into an array
    (bind _savetexta (`DialogLoader.FileLoadString` (`self.Dialog File`)))
    (set `self.DialogArray` (`KismetStringLibrary.ParseIntoArray` _savetexta ";"))
    ;[1 1 1] Set the first AI phrase
    (`TextBlock.SetText` (`self.TXT AIText`) (`KismetTextLibrary.Conv_StringToText` (`|GetArrayItem` (`self.DialogArray`) 1)))
    ;[1 1 1] Set initial first answer option for player (if answer is valid, otherwise hide the button)
    (if (!= _output_2 "-")
      (`TextBlock.SetText` (`self.TXT Char Choice 1`) (`KismetTextLibrary.Conv_StringToText` _output_2))
      (else
        (`/Game/Characters/Robots/AI_Components/dialogueTree/W_DialogueHUD.HideGUIWidget` (`self.DialogHud`) (`Widget.GetParent` (`self.TXT Char Choice 1`)))))
    ;[1 1 1] Set initial second answer for player...
    (if (!= _output_3 "-")
      (`TextBlock.SetText` (`self.TXT Char Choice 2`) (`KismetTextLibrary.Conv_StringToText` _output_3))
      (else
        (`/Game/Characters/Robots/AI_Components/dialogueTree/W_DialogueHUD.HideGUIWidget` (`self.DialogHud`) (`Widget.GetParent` (`self.TXT Char Choice 2`)))))
    ;[1 1 1] Set initial third answer for player...
    (if (!= _output "-")
      (`TextBlock.SetText` (`self.TXT Char Choice 3`) (`KismetTextLibrary.Conv_StringToText` _output))
      (else
        (`/Game/Characters/Robots/AI_Components/dialogueTree/W_DialogueHUD.HideGUIWidget` (`self.DialogHud`) (`Widget.GetParent` (`self.TXT Char Choice 3`)))))
    (set `self.CurrentAIPhraseID` 1)))

(fn `ShowAnswerGUIWidgets`
  (bind _dialoghud (`self.DialogHud`))
  (`/Game/Characters/Robots/AI_Components/dialogueTree/W_DialogueHUD.ShowGUIWidget` _dialoghud (`Widget.GetParent` (`/Game/Characters/Robots/AI_Components/dialogueTree/W_DialogueHUD.TXT_CharChoice1` _dialoghud)))
  (`/Game/Characters/Robots/AI_Components/dialogueTree/W_DialogueHUD.ShowGUIWidget` _dialoghud (`Widget.GetParent` (`/Game/Characters/Robots/AI_Components/dialogueTree/W_DialogueHUD.TXT_CharChoice2` _dialoghud)))
  (`/Game/Characters/Robots/AI_Components/dialogueTree/W_DialogueHUD.ShowGUIWidget` _dialoghud (`Widget.GetParent` (`/Game/Characters/Robots/AI_Components/dialogueTree/W_DialogueHUD.TXT_CharChoice3` _dialoghud))))

(fn `UpdateTree`
  (params (SelectedResponse :type Integer))
  (returns (ResponseTag :type String) (ResponseInfo :type String) (NextNode :type Integer))
  (bind _dialogarray (`self.DialogArray`))
  (bind _txt_char_choice_1 (`self.TXT Char Choice 1`))
  (bind _txt_char_choice_2 (`self.TXT Char Choice 2`))
  (bind _txt_char_choice_3 (`self.TXT Char Choice 3`))
  (bind _returnvalue (- (+ (* SelectedResponse 5) (* (`self.CurrentAIPhraseID`) 5)) 1))
  (bind _returnvalue_2 (`KismetStringLibrary.Conv_StringToInt` (`|GetArrayItem` (`self.DialogArray`) _returnvalue)))
  (bind _returnvalue_3 (- (* (`KismetStringLibrary.Conv_StringToInt` (`|GetArrayItem` (`self.DialogArray`) _returnvalue)) 5) 4))
  (bind _output (`|GetArrayItem` (`self.DialogArray`) (+ _returnvalue_3 15)))
  (bind _output_2 (`|GetArrayItem` (`self.DialogArray`) (+ _returnvalue_3 5)))
  (bind _output_3 (`|GetArrayItem` (`self.DialogArray`) (+ _returnvalue_3 10)))
  (`self.ShowAnswerGUIWidgets`)
  ;[1 1 1] Extract tag and info out of the discussion sentence
  (set `self.Tag` (`|GetArrayItem` _dialogarray (- _returnvalue 2)))
  (set `self.Info` (`|GetArrayItem` _dialogarray (- _returnvalue 1)))
  ;[1 1 1] Check if the conversation continues or not (AI index 0), if ends, return tag and info
  (if (> _returnvalue_2 0)
    ;[1 1 1] Continue with the conversation
    ;;[1 1 1] Get the next phrase and place it in the GUI
    (`TextBlock.SetText` (`self.TXT AIText`) (`KismetTextLibrary.Conv_StringToText` (`|GetArrayItem` (`self.DialogArray`) _returnvalue_3)))
    ;[1 1 1] Get players first option and place it in the GUI (if conversation continues)
    (if (!= _output_2 "-")
      (`TextBlock.SetText` _txt_char_choice_1 (`KismetTextLibrary.Conv_StringToText` _output_2))
      (else
        (`/Game/Characters/Robots/AI_Components/dialogueTree/W_DialogueHUD.HideGUIWidget` (`self.DialogHud`) (`Widget.GetParent` _txt_char_choice_1))))
    ;[1 1 1] Get players second option and place it in the GUI
    (if (!= _output_3 "-")
      (`TextBlock.SetText` _txt_char_choice_2 (`KismetTextLibrary.Conv_StringToText` _output_3))
      (else
        (`/Game/Characters/Robots/AI_Components/dialogueTree/W_DialogueHUD.HideGUIWidget` (`self.DialogHud`) (`Widget.GetParent` _txt_char_choice_2))))
    ;[1 1 1] Get players third option and place it in the GUI
    (if (!= _output "-")
      (`TextBlock.SetText` _txt_char_choice_3 (`KismetTextLibrary.Conv_StringToText` _output))
      (else
        (`/Game/Characters/Robots/AI_Components/dialogueTree/W_DialogueHUD.HideGUIWidget` (`self.DialogHud`) (`Widget.GetParent` _txt_char_choice_3))))
    ;[1 1 1] Update current AI phrase and return with ID if the conversation is over or not and what is outcome
    (bind _output_get (set `self.CurrentAIPhraseID` (`KismetStringLibrary.Conv_StringToInt` (`|GetArrayItem` (`self.DialogArray`) _returnvalue))))
    (return (`self.Tag`) (`self.Info`) _output_get)
    (else
      (return (`self.Tag`) (`self.Info`) _returnvalue_2))))