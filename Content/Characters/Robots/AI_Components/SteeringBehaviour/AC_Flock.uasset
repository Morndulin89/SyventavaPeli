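; Flocking steering component for robot AI (Daleks) that nudges a pawn's movement according to nearby flockmates.
; CalculateNewPosition gathers neighbours within a radius from the GameInstance's flocking list, then weights cohesion, alignment and separation into one direction.
; It lerps between that direction, flattened to the pawn's height, and the pawn's VelocityForFlocking by FlockingStrength, feeding the result to AddMovementInput.
; Debug lines visualise the steering vectors.
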(event `/Game/Characters/Robots/AI_Components/SteeringBehaviour/BI_SteeringBehaviourIndividual.calculateNewPosition`
  (params (ownCM :type "CharacterMovementComponent Object Reference"))
  (bind _myactorlocation (`self.MyActorLocation`))
  (bind _myactorlocation_2 (`self.MyActorLocation`))
  (bind _myactorlocation_3 (`self.MyActorLocation`))
  (bind _returnvalue (`Actor.K2_GetActorLocation` (`self.MyPawn`)))
  (set `self.MyPawn` (`PawnMovementComponent.GetPawnOwner` ownCM))
  ;[1 1 1] calculate new direction
  (`self.FindNeighbours`)
  (bind _cohesionresult (`self.CalculateCohesion`))
  (bind _alignment_result (`self.CalculateAlignment`))
  (bind _separationresult (`self.calculateSeparation`))
  (bind _newdiretion (`self.CalculateNewDirection` _cohesionresult _alignment_result _separationresult))
  ;[1 1 1] Find out where flocking suggests AI goes and draw debug line
  (set `self.MyActorLocation` _returnvalue)
  (bind _returnvalue_2 (`KismetMathLibrary.MakeVector` (.x (+ (* _newdiretion (`self.AmplifierValue`)) _returnvalue)) (.y (+ (* _newdiretion (`self.AmplifierValue`)) _returnvalue)) (.z _returnvalue)))
  (`KismetSystemLibrary.DrawDebugLine` _myactorlocation_2 (+ _myactorlocation_2 (* (`KismetMathLibrary.GetDirectionUnitVector` _myactorlocation_2 _returnvalue_2) (`self.AmplifierValue`))) (struct :`R` 1.0 :`B` 0.739549 :`A` 1.0))
  ;[1 1 1] Find out AI character's current own velocity despite of flocking and draw debug line
  (bind _asbp_dalek_flocking (cast `/Game/Characters/Robots/BP_DalekFlocking` (`self.MyPawn`)))
  (bind _returnvalue_3 (+ _myactorlocation_3 (* (`KismetMathLibrary.Normal` (`/Game/Characters/Robots/BP_DalekFlocking.velocityForFlocking` _asbp_dalek_flocking)) (`self.AmplifierValue`))))
  (`KismetSystemLibrary.DrawDebugLine` _myactorlocation_3 _returnvalue_3 (struct :`G` 0.966812 :`B` 1.0 :`A` 1.0))
  ;[1 1 1] calculate combination of flocking force and existing velocity and draw debug line
  (`KismetSystemLibrary.DrawDebugLine` _myactorlocation)
  (`Pawn.AddMovementInput` (`self.MyPawn`) (- (+ _myactorlocation (* (`KismetMathLibrary.GetDirectionUnitVector` (`self.MyActorLocation`) (`KismetMathLibrary.VLerp` _returnvalue_2 _returnvalue_3 (`self.FlockingStrength`))) (`self.AmplifierValue`))) (`self.MyActorLocation`)) 1.0 false))

(fn `CalculateAlignment`
  (returns (`Alignment result` :type "Vector Structure"))
  (locals (Alignment :type "Vector Structure" :default (0.0 0.0 0.0)))
  ;[1 1 1] Add velocity of neighbours into separation force
  (for _array_element (`self.Neighbours`)
    (bind _asbp_dalek_flocking (cast `/Game/Characters/Robots/BP_DalekFlocking` _array_element))
    (bind _output_get (set `local.Alignment` (+ (`local.Alignment`) (`/Game/Characters/Robots/BP_DalekFlocking.velocityForFlocking` _asbp_dalek_flocking)))))
  (return (`KismetMathLibrary.Normal` (/ _output_get (`KismetArrayLibrary.Array_Length` (`self.Neighbours`))))))

(fn `CalculateCohesion`
  (returns (cohesionResult :type "Vector Structure"))
  (locals (Cohesion :type "Vector Structure"))
  ;[1 1 1] add location of each neighbour into cohesion force
  (for _array_element (`self.Neighbours`)
    (bind _output_get (set `local.Cohesion` (+ (`Actor.K2_GetActorLocation` _array_element) (`local.Cohesion`))))
    (return (`KismetMathLibrary.Normal` (- (/ _output_get (`KismetArrayLibrary.Array_Length` (`self.Neighbours`))) (`Actor.K2_GetActorLocation` (`self.GetOwner`)))))))

(fn `CalculateNewDirection`
  (params (Cohesion :type "Vector Structure") (Alignment :type "Vector Structure") (Separation :type "Vector Structure"))
  (returns (NewDiretion :type "Vector Structure"))
  (locals (cohesionWeight :type "Float (double-precision)" :default 0.05) (alignmentWeight :type "Float (double-precision)" :default 0.9) (separationWeight :type "Float (double-precision)" :default 0.05) (amplifierValueNewDirection :type "Float (double-precision)" :default 3.0))
  (bind _cohesionweight (`local.cohesionWeight`))
  (bind _separationweight (`local.separationWeight`))
  (bind _alignmentweight (`local.alignmentWeight`))
  (return (`KismetMathLibrary.Normal` (/ (`KismetMathLibrary.MakeVector` (+ (+ (* _cohesionweight (.x Cohesion)) (* _alignmentweight (.x Alignment))) (* _separationweight (.x Separation))) (+ (+ (* _cohesionweight (.y Cohesion)) (* _alignmentweight (.y Alignment))) (* _separationweight (.y Separation))) (+ (+ (* _cohesionweight (.z Cohesion)) (* _alignmentweight (.z Alignment))) (* _separationweight (.z Separation)))) (`local.amplifierValueNewDirection`)))))

(fn `calculateSeparation`
  (returns (SeparationResult :type "Vector Structure"))
  (locals (Separation :type "Vector Structure" :default (20.0 20.0 0.0)))
  ;[1 1 1] Add direction towards each neighbour into separation force
  (for _array_element (`self.Neighbours`)
    (bind _output_get (set `local.Separation` (+ (`local.Separation`) (- (`Actor.K2_GetActorLocation` _array_element) (`Actor.K2_GetActorLocation` (`self.GetOwner`)))))))
  (return (`KismetMathLibrary.Normal` (`KismetMathLibrary.NegateVector` (/ _output_get (`KismetArrayLibrary.Array_Length` (`self.Neighbours`)))))))

(fn `FindNeighbours`
  (locals (NeighbourhoodRadius :type "Float (double-precision)" :default 10000.0))
  (bind _returnvalue (`self.GetOwner`))
  ;[1 1 1] Get all the AIcharacters and set them into the Flock-array
  (bind _asmy_game_instance (cast `/Game/MyGameInstance` (`GameplayStatics.GetGameInstance`)))
  (bind _output_get (set `self.Flock` (`/Game/MyGameInstance.flockingAICharacters` _asmy_game_instance)))
  ;[1 1 1] empty neighbours-array
  (`KismetArrayLibrary.Array_Clear` (`self.Neighbours`))
  (for _array_element _output_get
    ;[1 1 1] Check that array element is valid and not self
    (if (`KismetSystemLibrary.IsValid` _array_element)
      (if (!= _array_element _returnvalue)
        ;[1 1 1] check the distance of the array element to this AI character and if close enough, add it to this characters neighbours
        (if (< (`Actor.GetDistanceTo` _array_element _returnvalue) (`local.NeighbourhoodRadius`))
          (`KismetArrayLibrary.Array_Add` (`self.Neighbours`) _array_element))))))