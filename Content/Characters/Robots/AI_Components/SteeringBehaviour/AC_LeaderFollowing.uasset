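; Actor component for robot AI that implements leader-following steering, moving its pawn toward a point behind the target.
; Each CalculateNewPosition call gathers nearby characters from the GameInstance's flocking list and averages an amplified separation vector away from them.
; Arrival steers to the follow point, scaling movement input down inside a slowing radius.
; Both vectors are blended with a weighted lerp, then drive movement input and yaw-facing rotation.
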(event `/Game/Characters/Robots/AI_Components/SteeringBehaviour/BI_SteeringBehaviourRelational.calculateNewPosition`
  (params (ownCM :type "CharacterMovementComponent Object Reference") (targetCM :type "CharacterMovementComponent Object Reference"))
  (bind _output_get (set `self.Own CM` ownCM))
  ;[1 1 1] get the neighbours, calculate separation and arrival values and based on the two, the new direction
  (`self.FindNeighbours`)
  (bind _separationresult (`self.CalculateSeparation`))
  (bind _arrivalresult (`self.CalculateArrival` _output_get targetCM))
  (bind _newdirection (`self.CalculateNewDirection` _separationresult _arrivalresult))
  ;[1 1 1] Move the AI character
  (`Pawn.AddMovementInput` (`PawnMovementComponent.GetPawnOwner` (`self.Own CM`)) _newdirection (`self.ScaleValueForMovementInput`) false)
  ;[1 1 1] rotate towards movement direction (maybe not needed?)
  (`Actor.K2_SetActorRotation` (`PawnMovementComponent.GetPawnOwner` (`self.Own CM`)) (`KismetMathLibrary.Conv_VectorToRotator` (`KismetMathLibrary.MakeVector` (.x _newdirection) (.y _newdirection))) false))

(fn `CalculateArrival`
  (params (OwnCM :type "CharacterMovementComponent Object Reference") (TargetCM :type "CharacterMovementComponent Object Reference"))
  (returns (ArrivalResult :type "Vector Structure"))
  (locals (DistanceToLeader :type "Float (double-precision)" :default 80.0) (SlowingRadius :type "Float (double-precision)" :default 200.0))
  (bind _returnvalue (- (- (`CharacterMovementComponent.GetLastUpdateLocation` TargetCM) (* (`Actor.GetActorForwardVector` (`self.GetOwner` TargetCM)) (`local.DistanceToLeader`))) (`CharacterMovementComponent.GetLastUpdateLocation` (`self.Own CM`))))
  (bind _returnvalue_2 (/ (`KismetMathLibrary.NormalizeToRange` (`KismetMathLibrary.VSize` _returnvalue) 0.0 (`local.SlowingRadius`)) (`self.SlowingFactor`)))
  ;[1 1 1] Check if distance to target is above slowing radius
  (if (> (`KismetMathLibrary.Abs` (`KismetMathLibrary.VSize` _returnvalue)) (`local.SlowingRadius`))
    ;[1 1 1] Move towards player with original speed
    (set `self.ScaleValueForMovementInput` 1.0)
    (return (`KismetMathLibrary.VLerp` _returnvalue (`MovementComponent.Velocity` (`self.Own CM`)) 0.5))
    (else
      ;[1 1 1] Move towards the player with gradually slowing speed
      (if (>= _returnvalue_2 0.0)
        (set `self.ScaleValueForMovementInput` _returnvalue_2)
        (return _returnvalue)))))

(fn `CalculateNewDirection`
  (params (Separation :type "Vector Structure") (TargetDirection :type "Vector Structure"))
  (returns (NewDirection :type "Vector Structure"))
  (return (`KismetMathLibrary.VLerp` Separation TargetDirection 0.6)))

(fn `CalculateSeparation`
  (returns (separationResult :type "Vector Structure"))
  (locals (Separation :type "Vector Structure" :default (20.0 20.0 0.0)) (AmplifierSeparation :type Integer :default 300))
  (for _array_element (`self.Neighbours`)
    ;[1 1 1] Add direction towards each neighbour into separation force
    (bind _output_get (set `local.Separation` (+ (`local.Separation`) (- (`Actor.K2_GetActorLocation` _array_element) (`Actor.K2_GetActorLocation` (`self.GetOwner`)))))))
  (return (* (`KismetMathLibrary.Normal` (`KismetMathLibrary.NegateVector` (/ _output_get (`KismetArrayLibrary.Array_Length` (`self.Neighbours`))))) (`local.AmplifierSeparation`))))

(fn `FindNeighbours`
  ;[1 1 1] Get all relevant AI characters, set them as flock and clear previours neighbours
  (bind _asmy_game_instance (cast `/Game/MyGameInstance` (`GameplayStatics.GetGameInstance`)))
  (bind _output_get (set `self.Flock` (`/Game/MyGameInstance.flockingAICharacters` _asmy_game_instance)))
  (`KismetArrayLibrary.Array_Clear` (`self.Neighbours`))
  (for _array_element _output_get
    ;[1 1 1] Check array element is valid and not self
    (if (`KismetSystemLibrary.IsValid` _array_element)
      (if (!= _array_element (`self.GetOwner`))
        ;[1 1 1] Check if close enough, if true, add to neighbours of this character
        (if (< (`Actor.GetDistanceTo` _array_element null) (`self.FlockThreshold`))
          (`KismetArrayLibrary.Array_Add` (`self.Neighbours`) _array_element))))))