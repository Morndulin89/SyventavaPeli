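; Steering behaviour component for robot AI that patrols a path, but halts immediately whenever the target's movement component has non-zero velocity.
; CalculateNewPosition falls back to a default path if none is set, then advances to the next node within an arrival radius, reversing direction at either end.
; Movement input blends the vector to the current node slightly with the robot's own velocity.
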(event `/Game/Characters/Robots/AI_Components/SteeringBehaviour/BI_SteeringBehaviourRelational.calculateNewPosition`
  (params (ownCM :type "CharacterMovementComponent Object Reference") (targetCM :type "CharacterMovementComponent Object Reference"))
  (bind _currentnode (`self.CurrentNode`))
  (bind _own_cm (`self.Own CM`))
  (set `self.Own CM` ownCM)
  (if (> (`KismetMathLibrary.VSize` (`MovementComponent.Velocity` targetCM)) 0.0)
    (`MovementComponent.StopMovementImmediately` (`self.Own CM`))
    (else
      ;[1 1 1] Path following
      ;;[1 1 1] Get if the path has been set or not
      (if (not (> (`KismetArrayLibrary.Array_Length` (`self.Path`)) 0))
        ;;[1 1 1] If path has not been set, use default path
        (`self.setPath` (`self.DefaultPath`)))
      ;;[1 1 1] Get current node location on path
      (bind _output_get (set `self.Target` (`|GetArrayItem` (`self.Path`) (`self.CurrentNode`))))
      ;;[1 1 1] Check whether we have already reached the location
      (if (<= (`KismetMathLibrary.Vector_Distance` _output_get (`CharacterMovementComponent.GetLastUpdateLocation` (`self.Own CM`))) (`self.Radius`))
        ;;[1 1 1] If so, get next target node
        (set `self.CurrentNode` (+ (`self.CurrentNode`) (`self.PathDir`)))
        ;;[1 1 1] Check whether if it is the first or the last node
        (if (or (< _currentnode 0) (>= _currentnode (`KismetArrayLibrary.Array_Length` (`self.Path`))))
          ;;[1 1 1] If so, switch movement direction
          (set `self.PathDir` (* (`self.PathDir`) -1))
          (set `self.CurrentNode` (+ (`self.CurrentNode`) (`self.PathDir`)))))
      ;;[1 1 1] Get distance between player and target, substract AI character's velocity from it
      (`Pawn.AddMovementInput` (`PawnMovementComponent.GetPawnOwner` _own_cm) (`KismetMathLibrary.VLerp` (- (`self.Target`) (`CharacterMovementComponent.GetLastUpdateLocation` _own_cm)) (`MovementComponent.Velocity` _own_cm) 0.1) 1.0 false))))

(fn `setPath`
  (params (NewPath :type "Array of Vector Structure"))
  ;[1 1 1] Aseta kuljettava reitti
  (set `self.Path` NewPath))