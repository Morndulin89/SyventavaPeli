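; BP_Tardis is a player-controlled spaceship that constantly moves forward, steered by pitch, yaw and roll input, with its own HUD widget.
; Space or left mouse fires the Weapon; right mouse raises the Shield, then destroys it after five seconds.
; The construction script points Weapon, Shield and Recharger at a shared EnergySource.
; Any Box overlap reduces Health while it stays above a threshold; the Asteroid tag check is disconnected.
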(event `self.ReceiveBeginPlay`
  (bind _returnvalue (`|CreateWidget` "/Game/UI/W_SpaceHUD.W_SpaceHUD_C"))
  (bind _output_get (set `self.HUD` _returnvalue))
  (`UserWidget.AddToPlayerScreen` _output_get 0))

(event `self.ReceiveTick`
  (params (DeltaSeconds :type "Float (single-precision)"))
  (`self.AddMovementInput` (`self.GetActorForwardVector`)))

(event `InputAxis|LookUp`
  (params (AxisValue :type "Float (single-precision)"))
  (`self.AddControllerPitchInput` AxisValue))

(event `InputAxis|Turn`
  (params (AxisValue :type "Float (single-precision)"))
  (`self.AddControllerYawInput` AxisValue))

(event `InputAxis|Roll`
  (params (AxisValue :type "Float (single-precision)"))
  (`self.AddControllerRollInput` AxisValue))

(event `Key|SpaceBar`
  (params (Key :type "Key Structure"))
  (:`Pressed`
    (`Weapon.Shoot` (`self.Weapon`) :!label _label)))

(event `Key|LeftMouseButton`
  (params (Key :type "Key Structure"))
  (:`Pressed`
    (goto _label)))

(event `Key|RightMouseButton`
  (params (Key :type "Key Structure"))
  (bind _shield (`self.Shield`))
  (:`Pressed`
    (`Shield.Protect` _shield)
    (`KismetSystemLibrary.Delay` 5.0)
    (`Shield.DestroyShield` _shield)))

(event `self.Box.OnComponentBeginOverlap`
  (params (OverlappedComponent :type "PrimitiveComponent Object Reference") (OtherActor :type "Actor Object Reference") (OtherComp :type "PrimitiveComponent Object Reference") (OtherBodyIndex :type Integer) (bFromSweep :type Boolean) (SweepResult :type "HitResult Structure (by ref)"))
  ;[1 1 1] Why doesn't this work?
  (`KismetSystemLibrary.PrintString` "Asteroidcollided")
  (if (> (`self.Health`) 10.0)
    (set `self.Health` (- (`self.Health`) 10.0))))

(fn `UserConstructionScript`
  (set `EnergyConsumer.TargetSource` (`self.EnergySource`) (`self.Weapon`))
  (set `EnergyConsumer.TargetSource` (`self.EnergySource`) (`self.Shield`))
  (set `Recharger.TargetSource` (`self.EnergySource`) (`self.Recharger`)))