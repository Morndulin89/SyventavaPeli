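; Switch actor in the Station level's Security folder that toggles a state and animates its handle.
; It calls Toggle on BeginPlay and overrides the native event OnStateChanged, which only prints the new state in Finnish.
; UpdateVisualState plays a one-shot handle animation from State, SwitchOff when true and SwitchOn when false.
; Nothing in this graph calls UpdateVisualState.
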(event `self.ReceiveBeginPlay`
  (`self.Toggle`))

(event `self.OnStateChanged`
  (params (newState :type Boolean))
  (`KismetSystemLibrary.PrintString` (`KismetStringLibrary.Concat_StrStr` "Uusi tila on " (`KismetStringLibrary.Conv_BoolToString` newState))))

(fn `updateVisualState`
  (bind _handle (`self.handle`))
  (if (`self.state`)
    (`SkeletalMeshComponent.PlayAnimation` _handle "/Game/Levels/Station/Security/Graphics/ANIM_switch_handle_SwitchOff.ANIM_switch_handle_SwitchOff" false)
    (else
      (`SkeletalMeshComponent.PlayAnimation` _handle "/Game/Levels/Station/Security/Graphics/ANIM_switch_handle_SwitchOn.ANIM_switch_handle_SwitchOn" false))))

(fn `UserConstructionScript`)