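; BP_AirductCover is an interactable station airduct cover that the player can remove, after which a crawl prompt is shown.
; Interact hides the static mesh, disables its collision, sets CoverHasBeenRemoved and swaps the interact widget for the crawl widget.
; Box overlap begin and end show and hide the interact or crawl widget, chosen by that removed flag.
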(event `/Game/Levels/Interactables/InteractInterface.Interact`
  (bind _staticmesh (`self.StaticMesh`))
  ;[1 1 1] "Remove the airduct cover" (hide the mesh and remove collision)
  (`SceneComponent.SetVisibility` _staticmesh false false)
  (`PrimitiveComponent.SetCollisionEnabled` _staticmesh "NoCollision")
  (set `self.coverHasBeenRemoved` true)
  (`KismetSystemLibrary.PrintString` "cover removed")
  (`SceneComponent.SetVisibility` (`self.WidgetInteract`) false false)
  (`SceneComponent.SetVisibility` (`self.WidgetCrawl`) true false))

(event `self.Box.OnComponentBeginOverlap`
  (params (OverlappedComponent :type "PrimitiveComponent Object Reference") (OtherActor :type "Actor Object Reference") (OtherComp :type "PrimitiveComponent Object Reference") (OtherBodyIndex :type Integer) (bFromSweep :type Boolean) (SweepResult :type "HitResult Structure (by ref)"))
  ;[1 1 1] Only show the "interact with" text if the cover is in place
  (if (`self.coverHasBeenRemoved`)
    (`SceneComponent.SetVisibility` (`self.WidgetCrawl`) true false)
    (else
      (`SceneComponent.SetVisibility` (`self.WidgetInteract`) true false))))

(event `self.Box.OnComponentEndOverlap`
  (params (OverlappedComponent :type "PrimitiveComponent Object Reference") (OtherActor :type "Actor Object Reference") (OtherComp :type "PrimitiveComponent Object Reference") (OtherBodyIndex :type Integer))
  ;[1 1 1] Only show the "interact with" text if the cover is in place
  (if (`self.coverHasBeenRemoved`)
    (`SceneComponent.SetVisibility` (`self.WidgetCrawl`) false false)
    (else
      (`SceneComponent.SetVisibility` (`self.WidgetInteract`) false false))))

(fn `UserConstructionScript`)