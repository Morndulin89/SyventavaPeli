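; BP_Button is a floor button in the Station level that reacts to overlaps on its collision volume.
; Both begin and end overlap call Toggle and print State, then play or reverse a timeline.
; Timeline updates lerp the button mesh downward and set a dynamic material's emission and colour from State, lit when true and dim when false.
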(event `self.ReceiveBeginPlay`
  (bind _returnvalue (`PrimitiveComponent.CreateDynamicMaterialInstance` (`self.floorButton`) 0 "/Game/Levels/Station/Graphics/Materials/M_floorButton.M_floorButton" "None"))
  (set `self.floorBtnMaterial` _returnvalue))

(event `self.collision.OnComponentBeginOverlap`
  (params (OverlappedComponent :type "PrimitiveComponent Object Reference") (OtherActor :type "Actor Object Reference") (OtherComp :type "PrimitiveComponent Object Reference") (OtherBodyIndex :type Integer) (bFromSweep :type Boolean) (SweepResult :type "HitResult Structure (by ref)"))
  (bind _floorbtnmaterial (`self.floorBtnMaterial`))
  (`self.Toggle`)
  (`KismetSystemLibrary.PrintString` (`KismetStringLibrary.Concat_StrStr` "Btn state is " (`KismetStringLibrary.Conv_BoolToString` (`self.state`))))
  (bind (_direction _buttonheight) (`Timeline|Timeline` :!label _label)
    (:`Update`
      (`SceneComponent.K2_SetRelativeLocation` (`self.floorButton`) (`KismetMathLibrary.VLerp` (0.0 0.0 -5.0) (0.0 0.0 -10.0) _buttonheight) false false)
      (if (`self.state`)
        (`MaterialInstanceDynamic.SetScalarParameterValue` _floorbtnmaterial "EmissionStrength" 0.6)
        (`MaterialInstanceDynamic.SetVectorParameterValue` _floorbtnmaterial "ButtonColour" (struct :`R` 1.0 :`G` 1.0 :`B` 1.0 :`A` 1.0))
        (else
          (`MaterialInstanceDynamic.SetScalarParameterValue` _floorbtnmaterial "EmissionStrength" 0.1)
          (`MaterialInstanceDynamic.SetVectorParameterValue` _floorbtnmaterial "ButtonColour" (struct :`R` 0.229167 :`G` 0.229167 :`B` 0.229167 :`A` 1.0)))))))

(event `self.collision.OnComponentEndOverlap`
  (params (OverlappedComponent :type "PrimitiveComponent Object Reference") (OtherActor :type "Actor Object Reference") (OtherComp :type "PrimitiveComponent Object Reference") (OtherBodyIndex :type Integer))
  (`self.Toggle`)
  (`KismetSystemLibrary.PrintString` (`KismetStringLibrary.Concat_StrStr` "Btn state is " (`KismetStringLibrary.Conv_BoolToString` (`self.state`))))
  (goto _label :!via `Reverse`))

(fn `UserConstructionScript`)