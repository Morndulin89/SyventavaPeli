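; BP_Lever is an interactable lever for the Station level that flips its on/off state when used.
; Interact calls Toggle, prints the new state for debugging, then plays or reverses a timeline based on State.
; The timeline lerps the Scene component's pitch to swing the lever between its two angles.
; Box overlap events show and hide the interaction prompt widget.
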(event `/Game/Levels/Interactables/InteractInterface.Interact`
  (bind _state (`self.state`))
  ;[1 1 1] When interacted with, state changes via toggle and lever is turned
  (`self.Toggle`)
  (`KismetSystemLibrary.PrintString` (`KismetStringLibrary.Concat_StrStr` "Lever state is" (`KismetStringLibrary.Conv_BoolToString` _state)))
  (if _state
    ;;[1 1 1] Update the visual representation
    (bind (_direction _lever) (`Timeline|Timeline` :!via `Reverse` :!label _label)
      (:`Update`
        (`SceneComponent.K2_SetRelativeRotation` (`self.Scene`) (`KismetMathLibrary.MakeRotator` 0.0 (`KismetMathLibrary.Lerp` 50.0 -50.0 _lever)) false false)))
    (else
      (goto _label))))

(event `self.Box.OnComponentBeginOverlap`
  (params (OverlappedComponent :type "PrimitiveComponent Object Reference") (OtherActor :type "Actor Object Reference") (OtherComp :type "PrimitiveComponent Object Reference") (OtherBodyIndex :type Integer) (bFromSweep :type Boolean) (SweepResult :type "HitResult Structure (by ref)"))
  ;[1 1 1] Show/hide the interaction prompt
  (`SceneComponent.SetVisibility` (`self.Widget`) true false))

(event `self.Box.OnComponentEndOverlap`
  (params (OverlappedComponent :type "PrimitiveComponent Object Reference") (OtherActor :type "Actor Object Reference") (OtherComp :type "PrimitiveComponent Object Reference") (OtherBodyIndex :type Integer))
  ;[1 1 1] Show/hide the interaction prompt
  (`SceneComponent.SetVisibility` (`self.Widget`) false false))

(fn `UserConstructionScript`)