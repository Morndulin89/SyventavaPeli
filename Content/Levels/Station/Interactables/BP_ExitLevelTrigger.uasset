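; Level exit trigger actor for the Station interactables that moves the player to another level after a cutscene.
; When an actor tagged Player overlaps the Trigger component, it plays the assigned level sequence and binds to its finish event.
; When the sequence finishes, it opens the level named by LevelName.
; Without a valid sequence, the overlap does nothing and no level change occurs.
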(event `self.Trigger.OnComponentBeginOverlap`
  (params (OverlappedComponent :type "PrimitiveComponent Object Reference") (OtherActor :type "Actor Object Reference") (OtherComp :type "PrimitiveComponent Object Reference") (OtherBodyIndex :type Integer) (bFromSweep :type Boolean) (SweepResult :type "HitResult Structure (by ref)"))
  (bind _playablesequence (`self.PlayableSequence`))
  (bind _sequenceplayer (`LevelSequenceActor.SequencePlayer` _playablesequence))
  ;[1 1 1] Is player
  (if (`self.ActorHasTag` OtherActor "Player")
    ;[1 1 1] Sequence is set
    (if (`KismetSystemLibrary.IsValid` _playablesequence)
      ;[1 1 1] Play sequence
      (`MovieSceneSequencePlayer.Play` _sequenceplayer)
      (add `MovieSceneSequencePlayer.OnFinished` _sequenceplayer (delegate `Change level`)))))

(event `Change level`
  (`GameplayStatics.OpenLevel` (`self.Level Name`)))

(fn `UserConstructionScript`)