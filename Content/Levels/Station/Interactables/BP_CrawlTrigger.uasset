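; Crawl-passage trigger actor that puts the player into spline-following crawl movement between a start and end trigger.
; Overlapping TriggerStart sets IsCrawling on the tagged player and switches its CustomMovementComponent to custom SplineMovement mode, assigning this actor's Spline.
; Overlapping TriggerEnd clears the flag and spline and restores Walking.
; An unconnected alternative that moves the actor along the spline directly is left unused.
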(event `self.ReceiveTick`
  (params (DeltaSeconds :type "Float (single-precision)")))

(event `self.TriggerStart.OnComponentBeginOverlap`
  (params (OverlappedComponent :type "PrimitiveComponent Object Reference") (OtherActor :type "Actor Object Reference") (OtherComp :type "PrimitiveComponent Object Reference") (OtherBodyIndex :type Integer) (bFromSweep :type Boolean) (SweepResult :type "HitResult Structure (by ref)"))
  ;[1 1 1] When box is triggered, set player movement mode and set  bool
  (if (`self.ActorHasTag` OtherActor "Player")
    (bind _asbp_player_character (cast `/Game/Characters/PlayerCharacter/BP_PlayerCharacter` OtherActor))
    (set `/Game/Characters/PlayerCharacter/BP_PlayerCharacter.isCrawling` true _asbp_player_character) ; set is crawling
    (bind _charactermovement (`Character.CharacterMovement` _asbp_player_character))
    (`CharacterMovementComponent.SetMovementMode` _charactermovement "MOVE_Custom" (enumliteral `ECustomMovement` "MOVE_SplineMovement"))
    (bind _ascustom_movement_component (cast `CustomMovementComponent` _charactermovement))
    ;;[1 1 1] set spline
    (set `CustomMovementComponent.MovementSpline` (`self.Spline`) _ascustom_movement_component)))

(event `self.TriggerEnd.OnComponentBeginOverlap`
  (params (OverlappedComponent :type "PrimitiveComponent Object Reference") (OtherActor :type "Actor Object Reference") (OtherComp :type "PrimitiveComponent Object Reference") (OtherBodyIndex :type Integer) (bFromSweep :type Boolean) (SweepResult :type "HitResult Structure (by ref)"))
  ;[1 1 1] Move away from the spline
  (if (`self.ActorHasTag` OtherActor "Player")
    (bind _asbp_player_character (cast `/Game/Characters/PlayerCharacter/BP_PlayerCharacter` OtherActor))
    (set `/Game/Characters/PlayerCharacter/BP_PlayerCharacter.isCrawling` false _asbp_player_character) ; set is NOT crawling
    (bind _ascustom_movement_component (cast `CustomMovementComponent` (`Character.CharacterMovement` _asbp_player_character)))
    (`CharacterMovementComponent.SetMovementMode` _ascustom_movement_component "MOVE_Walking" 0)
    (set `CustomMovementComponent.MovementSpline` null _ascustom_movement_component)))

(fn `UserConstructionScript`)