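; BP_PushableBlock is an interactable station block that flags the player character as pushing.
; Two collision components, Y_AxisCollision and X_AxisCollision1, cast overlapping actors to BP_PlayerCharacter and set IsPushing.
; Both begin and end overlap events set IsPushing to true, so this Blueprint never clears the flag.
; The graph contains no movement logic, and the construction script is empty.
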(event `self.Y_AxisCollision.OnComponentBeginOverlap`
  (params (OverlappedComponent :type "PrimitiveComponent Object Reference") (OtherActor :type "Actor Object Reference") (OtherComp :type "PrimitiveComponent Object Reference") (OtherBodyIndex :type Integer) (bFromSweep :type Boolean) (SweepResult :type "HitResult Structure (by ref)"))
  ;[1 1 1] Update player character bool
  (bind _asbp_player_character (cast `/Game/Characters/PlayerCharacter/BP_PlayerCharacter` OtherActor))
  (set `/Game/Characters/PlayerCharacter/BP_PlayerCharacter.isPushing` true _asbp_player_character))

(event `self.Y_AxisCollision.OnComponentEndOverlap`
  (params (OverlappedComponent :type "PrimitiveComponent Object Reference") (OtherActor :type "Actor Object Reference") (OtherComp :type "PrimitiveComponent Object Reference") (OtherBodyIndex :type Integer))
  ;[1 1 1] Update player character bool
  (bind _asbp_player_character (cast `/Game/Characters/PlayerCharacter/BP_PlayerCharacter` OtherActor))
  (set `/Game/Characters/PlayerCharacter/BP_PlayerCharacter.isPushing` true _asbp_player_character))

(event `self.X_AxisCollision1.OnComponentBeginOverlap`
  (params (OverlappedComponent :type "PrimitiveComponent Object Reference") (OtherActor :type "Actor Object Reference") (OtherComp :type "PrimitiveComponent Object Reference") (OtherBodyIndex :type Integer) (bFromSweep :type Boolean) (SweepResult :type "HitResult Structure (by ref)"))
  ;[1 1 1] Update player character bool
  (bind _asbp_player_character (cast `/Game/Characters/PlayerCharacter/BP_PlayerCharacter` OtherActor))
  (set `/Game/Characters/PlayerCharacter/BP_PlayerCharacter.isPushing` true _asbp_player_character))

(event `self.X_AxisCollision1.OnComponentEndOverlap`
  (params (OverlappedComponent :type "PrimitiveComponent Object Reference") (OtherActor :type "Actor Object Reference") (OtherComp :type "PrimitiveComponent Object Reference") (OtherBodyIndex :type Integer))
  ;[1 1 1] Update player character bool
  (bind _asbp_player_character (cast `/Game/Characters/PlayerCharacter/BP_PlayerCharacter` OtherActor))
  (set `/Game/Characters/PlayerCharacter/BP_PlayerCharacter.isPushing` true _asbp_player_character))

(fn `UserConstructionScript`)