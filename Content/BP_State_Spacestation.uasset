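; Space station state Blueprint that runs a one-shot alarm countdown and kills the players when time runs out.
; ActivateTimer starts the countdown from AlarmTimeInSeconds only if no valid AlarmTimer handle exists, so repeat calls do not restart it.
; On expiry, PlayerDeath destroys every actor tagged "Player" and clears the timer handle inside that loop.
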(event `ActivateTimer`
  ;[1 1 1] Timer for game time remaining
  ;;[1 1 1] If NOT, create new timer
  ;;;[1 1 1] Check if there is already an alarm timer
  (if (not (`KismetSystemLibrary.K2_IsValidTimerHandle` (`self.AlarmTimer`)))
    (bind _returnvalue (`KismetSystemLibrary.K2_SetTimerDelegate` (delegate `PlayerDeath`) (`self.AlarmTimeInSeconds`)))
    (set `self.AlarmTimer` _returnvalue)))

(event `PlayerDeath`
  ;[1 1 1] When timer ends, destroy all actors with Player-tag and reset timer
  (bind _outactors (`GameplayStatics.GetAllActorsWithTag` "Player"))
  (for _array_element _outactors
    (`self.K2_DestroyActor` _array_element)
    (`KismetSystemLibrary.K2_ClearAndInvalidateTimerHandle` (`self.AlarmTimer`))))

(fn `UserConstructionScript`)